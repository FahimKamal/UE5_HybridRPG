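; Interactable NPC character that can roam the map and shows a dialogue indicator and a selection circle.
; When roaming, it loops AI moves to random nearby navigable points with random delays, pausing while interaction is locked.
; Starting an interaction hides the indicator and turns the NPC toward the instigator; ending it restores the indicator and resumes roaming.
; Selection shows the Target circle and starts a looping timer, apparently driving its spin-and-pulse animation, until deselected.
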(event `self.ReceiveBeginPlay`
  (`parent.ReceiveBeginPlay`)
  (`|ExecutionSequence`
    (:`then_0`
      (if (not (`self.IsInteractionAvailable`))
        (`SceneComponent.SetVisibility` (`self.DialogueIndicator`) false false)))
    (:`then_1`
      ;[0.0835 0.3542 0.06873 0.5] Walk to random location in the map in between delays
      (if (`self.IsRoaming`)
        (bind _randomlocation (`NavigationSystemV1.K2_GetRandomLocationInNavigableRadius` (`self.K2_GetActorLocation`) 1000.0 null null :!label _label))
        (`|AIMoveTo` self _randomlocation null 200.0
          (:`OnSuccess`
            _)
          (:`OnFail`
            _))
        (`self.Move Random with Delay`)))))

(event `Move Random with Delay`
  ;[0.0835 0.3542 0.06873 0.5] Walk to random location in the map in between delays
  (`KismetSystemLibrary.RetriggerableDelay` (`KismetMathLibrary.RandomFloatInRange` (`self.MinPatrolDelay`) (`self.MaxPatrolDelay`)))
  (if (not (`self.IsInteractionLocked`))
    (goto _label)))

(event `/Game/Blueprints/Interfaces/BPI_Interaction.StartInteraction`
  (params (InteractInstigator :type "Actor Object Reference"))
  (bind (_returnvalue_roll _returnvalue_pitch) (`KismetMathLibrary.BreakRotator` (`self.K2_GetActorRotation`)))
  (bind (_returnvalue_roll_2 _returnvalue_pitch_2 _returnvalue_yaw) (`KismetMathLibrary.BreakRotator` (`KismetMathLibrary.FindLookAtRotation` (`self.K2_GetActorLocation`) (`self.K2_GetActorLocation` InteractInstigator))))
  ;[0.0835 0.3542 0.06873 0.5] Interaction logic with player
  (`parent.StartInteraction` InteractInstigator)
  (`SceneComponent.SetVisibility` (`self.DialogueIndicator`) false false)
  (`/Engine/EditorBlueprintResources/StandardMacros.IsValid` InteractInstigator
    (:`Is Valid`
      ;;[0.4225 0.8388 0.8646 0.5] Make the Npc face the player at the time of interaction
      (`self.K2_SetActorRotation` (`KismetMathLibrary.MakeRotator` _returnvalue_roll _returnvalue_pitch _returnvalue_yaw)))))

(event `/Game/Blueprints/Interfaces/BPI_Interaction.EndInteraction`
  (`parent.EndInteraction`)
  (`SceneComponent.SetVisibility` (`self.DialogueIndicator`) true false)
  (if (`self.IsRoaming`)
    (`self.Move Random with Delay`)))

(event `self.ReceiveTick`
  (params (DeltaSeconds :type "Float (single-precision)"))
  (`parent.ReceiveTick` DeltaSeconds))

(event `AnimateTarget`
  ;[0.4225 0.8388 0.8646 0.5] Animate the circle
  ;;[0.5365 0.3663 0 0.5] Rotate the object
  (bind _output_get (set `self.ZRotation` (+ (`self.ZRotation`) 1.0)))
  (`SceneComponent.K2_SetRelativeRotation` (`self.Target`) (`KismetMathLibrary.MakeRotator` 0.0 0.0 _output_get) false false)
  (if (`self.Increase`)
    ;;[0.0835 0.3542 0.06873 0.5] Increase the size
    (if (<= (`self.TargetScale`) 1.4)
      (bind _output_get_2 (set `self.TargetScale` (+ (`self.TargetScale`) 0.005)))
      (`SceneComponent.SetRelativeScale3D` (`self.Target`) (`KismetMathLibrary.Conv_DoubleToVector` _output_get_2))
      (else
        (set `self.Increase` false)))
    (else
      ;;[0.5208 0.02167 0.02685 0.5] Decrease the size
      (if (>= (`self.TargetScale`) 1.0)
        (bind _output_get_3 (set `self.TargetScale` (- (`self.TargetScale`) 0.005)))
        (`SceneComponent.SetRelativeScale3D` (`self.Target`) (`KismetMathLibrary.Conv_DoubleToVector` _output_get_3))
        (else
          (set `self.Increase` true))))))

(event `Selected`
  ;[0.0835 0.3542 0.06873 0.5] Show the circle around the NPC.
  (`SceneComponent.SetVisibility` (`self.Target`) true false)
  (bind _returnvalue (`KismetSystemLibrary.K2_SetTimerDelegate` (`|CreateDelegate` :!event `AnimateTarget`) 0.05 true))
  (set `self.SelectedTimerHandle` _returnvalue))

(event `De-Selected`
  ;[0.5208 0.02167 0.02685 0.5] Hide the circle around the NPC>
  (`SceneComponent.SetVisibility` (`self.Target`) false false)
  (`KismetSystemLibrary.K2_ClearAndInvalidateTimerHandle` (`self.SelectedTimerHandle`)))

(fn `UserConstructionScript`
  (`parent.UserConstructionScript`))