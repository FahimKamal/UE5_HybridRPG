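; Player character Blueprint for an RPG, handling Enhanced Input movement along world X/Y and interaction with NPCs and objects.
; The interact input messages the first other actor overlapping InteractionCheck and stores it as LastInteracted.
; While interaction is locked, movement is blocked and the same input instantly reveals the HUD speech bubble's text or requests the next line.
; When no lines remain, it ends the interaction and hides the dialogue.
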(event `self.ReceiveBeginPlay`
  (`parent.ReceiveBeginPlay`)
  ;[0.0835 0.3542 0.06873 0.5] Initialize the inputs for player.
  (bind _asplayer_controller (cast `PlayerController` (`self.GetController`)))
  (`EnhancedInputSubsystemInterface.AddMappingContext` (pcsubsystem `EnhancedInputLocalPlayerSubsystem` _asplayer_controller) "/Game/Blueprints/Input/IMC_RPG.IMC_RPG" 0 (struct)))

(event `EnhancedInput|/Game/Blueprints/Input/Actions/IA_Move`
  (params (ActionValue :type "Vector2D Structure") (ElapsedSeconds :type "Float (double-precision)") (TriggeredSeconds :type "Float (double-precision)") (InputAction :type "InputAction Object Reference" :default "/Game/Blueprints/Input/Actions/IA_Move.IA_Move"))
  (bind (_x _y) (`KismetMathLibrary.BreakVector2D` ActionValue))
  ;[0.0835 0.3542 0.06873 0.5] Movement logic of player (W A S D) key to move around
  (:`Triggered`
    (if (not (`self.IsInteractionLocked`))
      (`self.AddMovementInput` (1.0 0.0 0.0) _x)
      (`self.AddMovementInput` (0.0 1.0 0.0) _y))))

(event `EnhancedInput|/Game/Blueprints/Input/Actions/IA_Interact`
  (params (ActionValue :type Boolean) (ElapsedSeconds :type "Float (double-precision)") (TriggeredSeconds :type "Float (double-precision)") (InputAction :type "InputAction Object Reference" :default "/Game/Blueprints/Input/Actions/IA_Interact.IA_Interact"))
  ;[0.0835 0.3542 0.06873 0.5] Full Interaction logic (E or Enter key)
  ;;[0.4225 0.8388 0.8646 0.5] Interaction logic with other NPC and objects. (E or Enter) key to Interact
  (:`Started`
    (if (`self.IsInteractionLocked`)
      (if (`/Game/Blueprints/Widgets/WBP_SpeechBubble.Finished Revealing` (`/Game/Blueprints/Widgets/WBP_HUD.WBP_SpeechBubble` (`self.HUDWidget`)))
        ;;[0.5365 0.3663 0 0.5] Check if there is more dialouge. If yes show it on screen.
        (bind _last_interacted (`self.Last Interacted`)
          (:`then`
            (bind _hasnextline (message `/Game/Blueprints/Interfaces/BPI_Interaction.ShowNextLIne` _last_interacted))
            (if (not _hasnextline)
              ;;[0.0835 0.3542 0.06873 0.5] False-> close the bubble.
              (`/Game/Blueprints/Interfaces/BPI_Interaction.EndInteraction`)
              (bind _last_interacted_2 (`self.Last Interacted`)
                (:`then`
                  (message `/Game/Blueprints/Interfaces/BPI_Interaction.EndInteraction` _last_interacted_2)
                  (`/Game/Blueprints/Widgets/WBP_HUD.HideDialogue` (`self.HUDWidget`)))
                (:`else`))))
          (:`else`))
        (else
          ;;[0.0835 0.3542 0.06873 0.5] False Reveal all latters at once.
          (`/Game/Blueprints/Widgets/WBP_SpeechBubble.Insta Reveal` (`/Game/Blueprints/Widgets/WBP_HUD.WBP_SpeechBubble` (`self.HUDWidget`)))))
      (else
        ;;[0.4225 0.8388 0.8646 0.5] Not in any interaction so start interaction.
        (for _array_element (`PrimitiveComponent.GetOverlappingActors` (`self.InteractionCheck`) null)
          (if (!= _array_element self)
            (message `/Game/Blueprints/Interfaces/BPI_Interaction.Interact` _array_element self)
            (set `self.Last Interacted` _array_element)
            (break)))))))

(fn `UserConstructionScript`
  (`parent.UserConstructionScript`))