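; BP_Follower is a character that trails the player pawn once an interaction with it ends.
; EndInteraction unlocks interaction, clears the current row name and starts FollowTarget.
; FollowTarget runs AI MoveTo toward the player within FollowDistance, then calls itself again on either success or failure, forming an endless follow loop.
; The follower-join 2D sound cue plays after each re-issued move, so it is not limited to the initial join.
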(event `/Game/Blueprints/Interfaces/BPI_Interaction.EndInteraction`
  (set `self.IsInteractionLocked` false)
  (set `self.Current Row Name` "None")
  (`self.Follow Target`))

(event `Follow Target`
  (`|AIMoveTo` self (0.0 0.0 0.0) (`GameplayStatics.GetPlayerPawn` 0) (`self.Follow Distance`)
    (:`OnSuccess`
      _)
    (:`OnFail`
      _))
  (`self.Follow Target`)
  (`GameplayStatics.PlaySound2D` "/Game/Sounds/S_Event_FollowerJoin_Cue.S_Event_FollowerJoin_Cue" 1.0 1.0 0.0 null null))

(fn `UserConstructionScript`
  (`parent.UserConstructionScript`))